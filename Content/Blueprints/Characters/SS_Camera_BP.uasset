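; Camera actor that becomes the first player controller's view target at a fixed rotation and follows the player character.
; A Tick state machine either snaps to the player, glides to a target actor for the "Draw Dridge" sequence, or glides back.
; Player control is disabled during that sequence and restored through a DoOnce, which resets once the camera returns to the player.
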(event Custom|StartEvent
  (params (Player_Ref :type Player%20Base%20CBP%20Object%20Reference))
  ;[1 1 1] Set view camera and set camera rotation
  (Variables|Default|SetPlayerBase_BP Player_Ref)
  (Game|Player|SetViewTargetwithBlend (Game|GetPlayerController 0) self 0.0 "VTBlend_Linear" 0.0 false)
  (Transformation|SetActorRotation "0,-90.000000, 0"))

(event EventTick
  (params (DeltaSeconds :type Float%20%28single-precision%29))
  ;[1 1 1] Camera states
  (switch Utilities|FlowControl|Switch|SwitchonCameraStates_Enum (Variables|Default|GetCameraStates)
    (:NewEnumerator2
      (Transformation|SetActorLocation (Transformation|GetActorLocation (Variables|Default|GetPlayerBase_BP)) false false)
      (Utilities|FlowControl|DoOnce false :!label _label
        (:Completed
          (Variables|/Game/Blueprints/Characters/PlayerBase_CBP.PlayerBase_CBP_C|SetCanControlPlayer? (Variables|Default|GetPlayerBase_BP) true))))
    (:NewEnumerator0
      (Variables|/Game/Blueprints/Characters/PlayerBase_CBP.PlayerBase_CBP_C|SetCanControlPlayer? (Variables|Default|GetPlayerBase_BP) false)
      (Transformation|SetActorLocation (Math|Interpolation|VInterpTo (Transformation|GetActorLocation) (Transformation|GetActorLocation (Variables|Default|GetActorToMoveto)) (Utilities|Time|GetWorldDeltaSeconds) 2.5) false false)
      (if (Math|Vector|Equal(Vector) (Transformation|GetActorLocation) (Transformation|GetActorLocation (Variables|Default|GetActorToMoveto)) 0.25)
        (Variables|Default|SetCameraStates "NewEnumerator3")))
    (:NewEnumerator3
      (Transformation|SetActorLocation (Math|Interpolation|VInterpTo (Transformation|GetActorLocation) (Transformation|GetActorLocation (Variables|Default|GetPlayerBase_BP)) (Utilities|Time|GetWorldDeltaSeconds) 2.5) false false)
      (if (Math|Vector|Equal(Vector) (Transformation|GetActorLocation) (Transformation|GetActorLocation (Variables|Default|GetPlayerBase_BP)) 0.25)
        (Variables|Default|SetCameraStates "NewEnumerator2")
        (goto _label Reset)))))

(fn ConstructionScript)