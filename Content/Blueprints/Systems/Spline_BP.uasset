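; Spline path actor that can chain onto a previous spline and displays colored arrows along its length.
; The construction script rebuilds the spline points in world space, snapping the first point to the last point of PreviousSpline when one is set.
; It then adds arrow static meshes at regular distance intervals, oriented along the spline direction, each tinted through a dynamic material instance.
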(event EventBeginPlay)

(event EventActorBeginOverlap
  (params (OtherActor :type Actor%20Object%20Reference)))

(event EventTick
  (params (DeltaSeconds :type Float%20%28single-precision%29)))

(fn ConstructionScript
  (bind _distancealongspline (Variables|Default|GetDistanceAlongSpline))
  (bind _spline (Variables|Default|GetSpline))
  (bind _previousspline (Variables|Default|GetPreviousSpline))
  (bind _spline_2 (Variables|Default|GetSpline))
  (bind _spline_3 (Variables|Spline_BP_C|GetSpline _previousspline))
  (Utilities|FlowControl|Sequence
    (:then_0
      ;[1 1 1] Set the array for the point
      (for _index (range 0 (- (Spline|GetNumberOfSplinePoints _spline_2) 1))
        (Utilities|Array|Add (Variables|Default|GetNewPoint) (Spline|GetLocationatSplinePoint _spline_2 _index "World")))
      (Utilities|FlowControl|Sequence
        (:then_0
          ;;[1 1 1] Set the position of the first point for the Spline to the position of the last point from the Previous Spline
          (if (!= _previousspline 0)
            (Utilities|Array|SetArrayElem (Variables|Default|GetNewPoint) 0 (Spline|GetLocationatSplinePoint _spline_3 (- (Spline|GetNumberOfSplinePoints _spline_3) 1) "World"))))
        (:then_1
          ;;[1 1 1] Set All the point
          (Spline|SetSplinePoints (Variables|Default|GetSpline) (Variables|Default|GetNewPoint) "World" true))))
    (:then_1
      ;[1 1 1] Create Arrow along the spline
      (for _index_2 (range 0 (Math|Float|Floor (/ (Spline|GetSplineLength _spline) _distancealongspline)))
        (bind _returnvalue (AddComponent|AddStaticMeshComponent false (Math|Transform|MakeTransform "0, 0, 0" "0, 0, 0" (Math|Conversions|ToVector(Float) (Variables|Default|GetArrowScale)))))
        (Transformation|SetWorldLocationAndRotation _returnvalue (Spline|GetLocationatDistanceAlongSpline _spline (Math|Conversions|ToFloat(Integer) (* _index_2 (Math|Float|Truncate _distancealongspline))) "World") (Math|Conversions|RotationFromXVector (Spline|GetDirectionatDistanceAlongSpline _spline (Math|Conversions|ToFloat(Integer) (* _index_2 (Math|Float|Truncate _distancealongspline))) "World")) false false)
        (bind _returnvalue_2 (Rendering|Material|CreateDynamicMaterialInstance _returnvalue 0 0 :!class /Script/Engine.PrimitiveComponent))
        (Rendering|Material|SetVectorParameterValue _returnvalue_2 "BaseColor" (Variables|Default|GetArrowColor) :!class /Script/Engine.MaterialInstanceDynamic)
        (Utilities|Array|Add (Variables|Default|GetArrowARRAY) _returnvalue)))))