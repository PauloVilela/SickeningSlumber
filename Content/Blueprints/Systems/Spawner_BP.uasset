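; Enemy spawner that fills a trigger volume's area with random AI enemies in the Nightmare world and removes enemies in the Dream world.
; The player's first Nightmare overlap of the construction-sized box spawns a batch at the actor's location and caches the player.
; ChangingWorlds saves every enemy's location and destroys it for Dream, then respawns at saved locations for Nightmare.
; Class, behavior tree and saved location use separate random indices, all ranged on EnemyTypes' length.
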(event OnComponentBeginOverlap(SpawnVolume)
  (params (OverlappedComponent :type Primitive%20Component%20Object%20Reference) (OtherActor :type Actor%20Object%20Reference) (OtherComp :type Primitive%20Component%20Object%20Reference) (OtherBodyIndex :type Integer) (bFromSweep :type Boolean) (SweepResult :type Hit%20Result%20Structure%20%28by%20ref%29))
  (bind _enemytypes (Variables|Default|GetEnemyTypes))
  (bind _returnvalue (Utilities|Array|Length _enemytypes))
  (bind _returnvalue_2 (Math|Random|RandomIntegerinRange 0 _returnvalue))
  (bind _asplayer_base_cbp (Utilities|Casting|CastToPlayerBase_CBP OtherActor))
  (bind _output_get (Variables|Default|SetPlayerBase_CBP _asplayer_base_cbp))
  (switch Utilities|FlowControl|Switch|SwitchonWorldType_Enum (Variables|/Game/Blueprints/Characters/PlayerBase_CBP.PlayerBase_CBP_C|GetWorldType _output_get)
    (:NewEnumerator1
      (Utilities|FlowControl|DoOnce false
        (:Completed
          (for _index (range 1 (Variables|SpawnerProperties|GetNumberOfEnemiesToSpawn))
            (AI|SpawnAIFromClass (Utilities|Array|Get(acopy) _enemytypes _returnvalue_2) (Utilities|Array|Get(acopy) (Variables|Default|GetEnemyBT) _returnvalue_2) (Transformation|GetActorLocation) "0, 0, 0" true))
          (Development|PrintString (Utilities|String|ToString(Integer) (Utilities|Array|Length (Variables|Default|GetEnemiesAdded)))))))))

(event Custom|ChangingWorlds
  (bind _enemytypes (Variables|Default|GetEnemyTypes))
  (bind _playerbase_cbp (Variables|Default|GetPlayerBase_CBP))
  (bind _returnvalue (Utilities|Array|Length _enemytypes))
  (bind _returnvalue_2 (Math|Random|RandomIntegerinRange 0 _returnvalue))
  (Utilities|IsValid _playerbase_cbp
    (:Is%20Valid
      (switch Utilities|FlowControl|Switch|SwitchonWorldType_Enum (Variables|/Game/Blueprints/Characters/PlayerBase_CBP.PlayerBase_CBP_C|GetWorldType _playerbase_cbp)
        (:NewEnumerator0
          (bind _outactors (Actor|GetAllActorsOfClass "/Game/Blueprints/Enemies/EnemyBase_BP.EnemyBase_BP_C"))
          (for _array_element _outactors
            (Utilities|IsValid _array_element
              (:Is%20Valid
                (Utilities|Array|Add (Variables|Default|GetLastKnowLocation) (Transformation|GetActorLocation _array_element))
                (Actor|DestroyActor _array_element)))))
        (:NewEnumerator1
          (for _index (range 1 (Variables|SpawnerProperties|GetNumberOfEnemiesToSpawn))
            (AI|SpawnAIFromClass (Utilities|Array|Get(acopy) _enemytypes _returnvalue_2) (Utilities|Array|Get(acopy) (Variables|Default|GetEnemyBT) _returnvalue_2) (Utilities|Array|Get(acopy) (Variables|Default|GetLastKnowLocation) _returnvalue_2) "0, 0, 0" true)))))))

(fn ConstructionScript
  (Components|Box|SetBoxExtent (Variables|Default|GetSpawnVolume) (Variables|SpawnerProperties|GetSpanVolumeScale) true))