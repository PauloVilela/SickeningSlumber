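; Main menu mesh actor that shows highlighting for its Play, Control and Quit options, each drawn by its own material slot on one static mesh.
; Paired toggle and remove events per option switch that slot's Colour scalar parameter on or off.
; Each call creates a new dynamic material instance from the slot's current material and stores it in a single shared DynamicMaterial variable.
; The events have no callers in this Blueprint.
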(event Custom|PlayTogger
  (bind _staticmeshcomponent (Variables|Debug|GetStaticMeshComponent))
  (bind _returnvalue (Rendering|Material|CreateDynamicMaterialInstance _staticmeshcomponent 0 (Rendering|Material|GetMaterial _staticmeshcomponent 0) :!class /Script/Engine.PrimitiveComponent))
  (bind _output_get (Variables|Default|SetDynamicMaterial _returnvalue))
  (Rendering|Material|SetScalarParameterValue (Variables|Default|GetDynamicMaterial) "Colour" 1.0 :!class /Script/Engine.MaterialInstanceDynamic))

(event Custom|QuitRemove
  (bind _staticmeshcomponent (Variables|Debug|GetStaticMeshComponent))
  (bind _returnvalue (Rendering|Material|CreateDynamicMaterialInstance _staticmeshcomponent 2 (Rendering|Material|GetMaterial _staticmeshcomponent 2) :!class /Script/Engine.PrimitiveComponent))
  (bind _output_get (Variables|Default|SetDynamicMaterial _returnvalue))
  (Rendering|Material|SetScalarParameterValue (Variables|Default|GetDynamicMaterial) "Colour" 0.0 :!class /Script/Engine.MaterialInstanceDynamic))

(event Custom|PlayRemove
  (bind _staticmeshcomponent (Variables|Debug|GetStaticMeshComponent))
  (bind _returnvalue (Rendering|Material|CreateDynamicMaterialInstance _staticmeshcomponent 0 (Rendering|Material|GetMaterial _staticmeshcomponent 0) :!class /Script/Engine.PrimitiveComponent))
  (bind _output_get (Variables|Default|SetDynamicMaterial _returnvalue))
  (Rendering|Material|SetScalarParameterValue (Variables|Default|GetDynamicMaterial) "Colour" 0.0 :!class /Script/Engine.MaterialInstanceDynamic))

(event Custom|ControlTogel
  (bind _staticmeshcomponent (Variables|Debug|GetStaticMeshComponent))
  (bind _returnvalue (Rendering|Material|CreateDynamicMaterialInstance _staticmeshcomponent 1 (Rendering|Material|GetMaterial _staticmeshcomponent 1) :!class /Script/Engine.PrimitiveComponent))
  (bind _output_get (Variables|Default|SetDynamicMaterial _returnvalue))
  (Rendering|Material|SetScalarParameterValue (Variables|Default|GetDynamicMaterial) "Colour" 1.0 :!class /Script/Engine.MaterialInstanceDynamic))

(event Custom|ControlRemove
  (bind _staticmeshcomponent (Variables|Debug|GetStaticMeshComponent))
  (bind _returnvalue (Rendering|Material|CreateDynamicMaterialInstance _staticmeshcomponent 1 (Rendering|Material|GetMaterial _staticmeshcomponent 1) :!class /Script/Engine.PrimitiveComponent))
  (bind _output_get (Variables|Default|SetDynamicMaterial _returnvalue))
  (Rendering|Material|SetScalarParameterValue (Variables|Default|GetDynamicMaterial) "Colour" 0.0 :!class /Script/Engine.MaterialInstanceDynamic))

(event Custom|QuitTogel
  (bind _staticmeshcomponent (Variables|Debug|GetStaticMeshComponent))
  (bind _returnvalue (Rendering|Material|CreateDynamicMaterialInstance _staticmeshcomponent 2 (Rendering|Material|GetMaterial _staticmeshcomponent 2) :!class /Script/Engine.PrimitiveComponent))
  (bind _output_get (Variables|Default|SetDynamicMaterial _returnvalue))
  (Rendering|Material|SetScalarParameterValue (Variables|Default|GetDynamicMaterial) "Colour" 1.0 :!class /Script/Engine.MaterialInstanceDynamic))

(fn ConstructionScript)