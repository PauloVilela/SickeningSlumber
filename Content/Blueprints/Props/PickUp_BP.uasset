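; PickUp_BP is a pickup prop that can be grabbed, dropped and placed at an attach point through an InsertKey event.
; Grab turns actor collision off, and Drop restores it, then enables physics on BaseModel after a short delay.
; Hitting anything other than the player character switches physics off again, so a dropped item freezes on impact.
; InsertKey moves the actor to the supplied position and rotation and prints a debug message.
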(event OnComponentHit(BaseModel)
  (params (HitComponent :type Primitive%20Component%20Object%20Reference) (OtherActor :type Actor%20Object%20Reference) (OtherComp :type Primitive%20Component%20Object%20Reference) (NormalImpulse :type Vector :default "0, 0, 0") (Hit :type Hit%20Result%20Structure%20%28by%20ref%29))
  (Utilities|Casting|CastToPlayerBase_CBP OtherActor
    (:CastFailed
      (Physics|SetSimulatePhysics (Variables|Default|GetBaseModel) false))))

(event Custom|Grab
  (Collision|SetActorEnableCollision self false))

(event Custom|InsertKey
  (params (AttachPosition :type Vector) (AttachRotation :type Rotator))
  (Transformation|SetActorLocationAndRotation AttachPosition AttachRotation)
  (Development|PrintString "PLACE"))

(event Custom|Drop
  (Collision|SetActorEnableCollision self true)
  (Utilities|FlowControl|Delay 0.1)
  (Physics|SetSimulatePhysics (Variables|Default|GetBaseModel) true))

(fn ConstructionScript)