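; EnemyBase_BP is a base enemy Blueprint that triggers chasing of the player and deals attack damage.
; On BeginPlay it caches a PlayerBase_CBP actor, then checks its distance every Tick and sets the "Chase?" Blackboard key when it is within a fixed range, never clearing it here.
; An Attack event switches on EnemyType, with only the Ghost case calling the player's TakeDamageInCombat.
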(event Custom|Attack
  (bind _player (Variables|Default|GetPlayer))
  (switch Utilities|FlowControl|Switch|SwitchonEnemyTypes_Enum (Variables|Default|GetEnemyType)
    (:NewEnumerator2
      (Utilities|IsValid _player
        (:Is%20Valid
          (Default|TakeDamageinCombat _player))))))

(event EventTick
  (params (DeltaSeconds :type Float%20%28single-precision%29))
  (bind _returnvalue (AI|GetBlackboard 0))
  (bind _player (Variables|Default|GetPlayer))
  ;[1 1 1] Overlap move to player
  (Utilities|IsValid _player
    (:Is%20Valid
      (Math|Float|CompareFloat (Transformation|GetDistanceTo _player self) 512.0
        (:<
          (Utilities|IsValid _returnvalue
            (:Is%20Valid
              (AI|Components|Blackboard|SetValueasBool _returnvalue (Utilities|Name|MakeLiteralName "Chase?") true))))))))

(event EventBeginPlay
  ;[1 1 1] On Start
  (bind _outactors (Actor|GetAllActorsOfClass "/Game/Blueprints/Characters/PlayerBase_CBP.PlayerBase_CBP_C"))
  (for _array_element _outactors
    (Variables|Default|SetPlayer _array_element)))

(fn ConstructionScript)